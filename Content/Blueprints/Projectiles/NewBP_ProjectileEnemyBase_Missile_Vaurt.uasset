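; Enemy homing missile projectile that chases the player pawn and self-destructs on a timer.
; BeginPlay runs the parent logic, turns on strong ProjectileMovement homing toward the player's root, then after a short delay spawns a large explosion and destroys the actor.
; A Box overlap with the player's secondary projectile destroys it early, as does any StaticMesh1 hit, both without an explosion.
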(event OnComponentBeginOverlap(Box)
  (params (OverlappedComponent :type Primitive%20Component%20Object%20Reference) (OtherActor :type Actor%20Object%20Reference) (OtherComp :type Primitive%20Component%20Object%20Reference) (OtherBodyIndex :type Integer) (bFromSweep :type Boolean) (SweepResult :type Hit%20Result%20Structure%20%28by%20ref%29))
  (Utilities|Casting|CastToBP_ProjectilePlayerSecondary OtherActor)
  (Actor|DestroyActor))

(event OnComponentHit(Box)
  (params (HitComponent :type Primitive%20Component%20Object%20Reference) (OtherActor :type Actor%20Object%20Reference) (OtherComp :type Primitive%20Component%20Object%20Reference) (NormalImpulse :type Vector :default "0, 0, 0") (Hit :type Hit%20Result%20Structure%20%28by%20ref%29)))

(event OnComponentHit(StaticMesh1)
  (params (HitComponent :type Primitive%20Component%20Object%20Reference) (OtherActor :type Actor%20Object%20Reference) (OtherComp :type Primitive%20Component%20Object%20Reference) (NormalImpulse :type Vector :default "0, 0, 0") (Hit :type Hit%20Result%20Structure%20%28by%20ref%29))
  (Utilities|Casting|CastToBP_ProjectilePlayerSecondary OtherActor
    (:then
      (Actor|DestroyActor))
    (:CastFailed
      (Actor|DestroyActor))))

(event EventBeginPlay
  (bind _projectilemovement (Variables|Default|GetProjectileMovement))
  (|CallParentFunction)
  (Variables|/Script/Engine.ProjectileMovementComponent|SetHomingTargetComponent _projectilemovement (Variables|/Script/Engine.Actor|GetRootComponent (Game|Player|GetPlayerPawn 0)))
  (Variables|/Script/Engine.ProjectileMovementComponent|SetbIsHomingProjectile _projectilemovement true)
  (Variables|/Script/Engine.ProjectileMovementComponent|SetHomingAccelerationMagnitude _projectilemovement 3e+04)
  (Utilities|FlowControl|Delay 3.0)
  (Effects|SpawnEmitteratLocation "/Game/Assets/Particles/Lea_particles/Explosion_small/P_Explosion_small.P_Explosion_small" (Transformation|GetActorLocation) "0, 0, 0" "100.000000,100.000000,100.000000")
  (Actor|DestroyActor))

(fn ConstructionScript
  (|CallParentFunction))