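; BP_Post_Test_pilot is a child Blueprint for a pilot post that enables piloting of a referenced Ship.
; Each tick, while the post is taken, it sets the Ship's pilot-active flag for player one or player two, based on PlayerOne.
; While the post is free, it clears both flags, stops the Ship's movement and cancels its roll-left and roll-right timers.
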(event EventBeginPlay
  (|CallParentFunction) ; This node is disabled and will not be called.\nDrag off pins to build functionality.
)

(event Collision|EventActorBeginOverlap
  (params (OtherActor :type Actor%20Object%20Reference))
  (|CallParentFunction OtherActor) ; This node is disabled and will not be called.\nDrag off pins to build functionality.
)

(event EventTick
  (params (DeltaSeconds :type Float%20%28single-precision%29))
  (bind _ship (Variables|Default|GetShip))
  (|CallParentFunction DeltaSeconds)
  (if (Variables|Default|GetisTaken)
    (if (Variables|Default|GetplayerOne?)
      (Variables|/Game/Blueprints/BP_Player.BP_Player_C|SetPilotActive _ship true)
      (else
        (Variables|/Game/Blueprints/BP_Player.BP_Player_C|SetPilotActive_P2 _ship true)))
    (else
      (Variables|/Game/Blueprints/BP_Player.BP_Player_C|SetPilotActive _ship false)
      (Variables|/Game/Blueprints/BP_Player.BP_Player_C|SetPilotActive_P2 _ship false)
      (Class|NavMovementComponent|StopActiveMovement (Variables|/Game/Blueprints/BP_Player.BP_Player_C|GetFloatingPawnMovement1 _ship))
      (Utilities|Time|ClearTimerbyFunctionName _ship "ShipRollRight")
      (Utilities|Time|ClearTimerbyFunctionName _ship "ShipRollLeft"))))

(fn ConstructionScript
  (|CallParentFunction))