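; Player post for the ship's left gatling gun, built as a child of a parent post Blueprint.
; Each tick it runs the parent logic, then while the post is taken it sets the Ship's left-gatling active flag for player one or player two.
; While the post is free it clears both flags and cancels the Ship's firing and gun-rotation timers by function name every tick.
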(event EventBeginPlay
  (|CallParentFunction) ; This node is disabled and will not be called.\nDrag off pins to build functionality.
)

(event Collision|EventActorBeginOverlap
  (params (OtherActor :type Actor%20Object%20Reference))
  (|CallParentFunction OtherActor) ; This node is disabled and will not be called.\nDrag off pins to build functionality.
)

(event EventTick
  (params (DeltaSeconds :type Float%20%28single-precision%29))
  (bind _ship (Variables|Default|GetShip))
  (|CallParentFunction DeltaSeconds)
  (if (Variables|Default|GetisTaken)
    (if (Variables|Default|GetplayerOne?)
      (Variables|/Game/Blueprints/Main_Character_OR_SpaceShip/Player/BP_Player.BP_Player_C|SetGatlingLeftActive _ship true)
      (else
        (Variables|/Game/Blueprints/Main_Character_OR_SpaceShip/Player/BP_Player.BP_Player_C|SetGatlingLeftActive_P2 _ship true)))
    (else
      (Variables|/Game/Blueprints/Main_Character_OR_SpaceShip/Player/BP_Player.BP_Player_C|SetGatlingLeftActive _ship false)
      (Variables|/Game/Blueprints/Main_Character_OR_SpaceShip/Player/BP_Player.BP_Player_C|SetGatlingLeftActive_P2 _ship false)
      (Utilities|Time|ClearTimerbyFunctionName _ship "SecFire")
      (Utilities|Time|ClearTimerbyFunctionName _ship "RotateGun")
      (Utilities|Time|ClearTimerbyFunctionName _ship "RotateLeftGatling1")
      (Utilities|Time|ClearTimerbyFunctionName _ship "RotateLeftGatling2"))))

(fn ConstructionScript
  (|CallParentFunction))