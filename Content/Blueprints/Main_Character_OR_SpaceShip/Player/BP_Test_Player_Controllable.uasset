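; Test controllable player character that takes and leaves posts on a ship, with a flag separating player one from player two.
; Toggling releases the current post, or searches the ship's post list for free ones within activation range and claims them for that player.
; Two chained timelines then slide the character to the post, keeping its height, and turn it to the post's facing.
; Switch Post and Z input toggle only for player two.
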(event Custom|Move%20To%20Post
  (bind _self self)
  (bind _currentpost (Variables|Default|GetcurrentPost))
  (bind _returnvalue (Transformation|GetActorLocation _self))
  (bind _returnvalue_2 (Transformation|GetActorLocation _currentpost))
  (bind _newtrack_0 (Timeline|moveToPostTL PlayFromStart)
    (:Update
      (Transformation|SetActorLocation (Math|Vector|Lerp(Vector) (Math|Vector|MakeVector (.x _returnvalue) (.y _returnvalue) (.z _returnvalue)) (Math|Vector|MakeVector (.x _returnvalue_2) (.y _returnvalue_2) (.z _returnvalue)) _newtrack_0) false false))
    (:Finished
      (bind _newtrack_0_2 (Timeline|Timeline_0 PlayFromStart)
        (:Update
          (Transformation|SetActorRotation (Math|Rotator|Lerp(Rotator) (Transformation|GetActorRotation self) (Math|Conversions|RotationFromXVector (Math|Vector|GetForwardVector (Variables|/Game/Blueprints/Main_Character_OR_SpaceShip/Player/BP_Post_Test.BP_Post_Test_C|GetCube (Variables|Default|GetcurrentPost)))) _newtrack_0_2)))))))

(event Custom|ayyyy
  (if (Variables|Default|GetusingPost)
    (Variables|Default|SetusingPost false)
    (Utilities|IsValid (Variables|Default|GetcurrentPost)
      (:Is%20Valid
        (Variables|/Game/Blueprints/Main_Character_OR_SpaceShip/Player/BP_Post_Test.BP_Post_Test_C|SetisTaken (Variables|Default|GetcurrentPost) false)
        (Variables|/Game/Blueprints/Main_Character_OR_SpaceShip/Player/BP_Post_Test.BP_Post_Test_C|SetplayerOne? (Variables|Default|GetcurrentPost) false)
        (Variables|/Game/Blueprints/Main_Character_OR_SpaceShip/Player/BP_Post_Test.BP_Post_Test_C|SetplayerTwo? (Variables|Default|GetcurrentPost) false)))
    (else
      (for _array_element (Variables|/Game/Blueprints/Main_Character_OR_SpaceShip/Player/BP_Player.BP_Player_C|GetPostList (Variables|Default|GetShip))
        (if (and (not (Variables|/Game/Blueprints/Main_Character_OR_SpaceShip/Player/BP_Post_Test.BP_Post_Test_C|GetisTaken _array_element)) (< (Math|Vector|VectorLength (- (Transformation|GetActorLocation _array_element) (Transformation|GetActorLocation self))) (Variables|Default|GetpostActivationDistance)))
          (bind _output_get (Variables|Default|SetcurrentPost _array_element))
          (Variables|/Game/Blueprints/Main_Character_OR_SpaceShip/Player/BP_Post_Test.BP_Post_Test_C|SetisTaken _output_get true)
          (CallFunction|MovetoPost)
          (Variables|Default|SetusingPost true)
          (if (Variables|Default|GetplayerOne?)
            (Variables|/Game/Blueprints/Main_Character_OR_SpaceShip/Player/BP_Post_Test.BP_Post_Test_C|SetplayerOne? _output_get true)
            (else
              (Variables|/Game/Blueprints/Main_Character_OR_SpaceShip/Player/BP_Post_Test.BP_Post_Test_C|SetplayerTwo? _output_get true))))))))

(event Custom|pleeeeasee
  (if (not (Variables|Default|GetplayerOne?))
    (if (Variables|Default|GetusingPost)
      (Variables|Default|SetusingPost false)
      (Utilities|IsValid (Variables|Default|GetcurrentPost)
        (:Is%20Valid
          (Variables|/Game/Blueprints/Main_Character_OR_SpaceShip/Player/BP_Post_Test.BP_Post_Test_C|SetisTaken (Variables|Default|GetcurrentPost) false)
          (Variables|/Game/Blueprints/Main_Character_OR_SpaceShip/Player/BP_Post_Test.BP_Post_Test_C|SetplayerOne? (Variables|Default|GetcurrentPost) false)
          (Variables|/Game/Blueprints/Main_Character_OR_SpaceShip/Player/BP_Post_Test.BP_Post_Test_C|SetplayerTwo? (Variables|Default|GetcurrentPost) false)))
      (else
        (for _array_element (Variables|/Game/Blueprints/Main_Character_OR_SpaceShip/Player/BP_Player.BP_Player_C|GetPostList (Variables|Default|GetShip))
          (if (and (not (Variables|/Game/Blueprints/Main_Character_OR_SpaceShip/Player/BP_Post_Test.BP_Post_Test_C|GetisTaken _array_element)) (< (Math|Vector|VectorLength (- (Transformation|GetActorLocation _array_element) (Transformation|GetActorLocation self))) (Variables|Default|GetpostActivationDistance)))
            (bind _output_get (Variables|Default|SetcurrentPost _array_element))
            (Variables|/Game/Blueprints/Main_Character_OR_SpaceShip/Player/BP_Post_Test.BP_Post_Test_C|SetisTaken _output_get true)
            (CallFunction|MovetoPost)
            (Variables|Default|SetusingPost true)
            (if (Variables|Default|GetplayerOne?)
              (Variables|/Game/Blueprints/Main_Character_OR_SpaceShip/Player/BP_Post_Test.BP_Post_Test_C|SetplayerOne? _output_get true)
              (else
                (Variables|/Game/Blueprints/Main_Character_OR_SpaceShip/Player/BP_Post_Test.BP_Post_Test_C|SetplayerTwo? _output_get true)))))))))

(event EventBeginPlay
  (|CallParentFunction) ; This node is disabled and will not be called.\nDrag off pins to build functionality.
)

(event Collision|EventActorBeginOverlap
  (params (OtherActor :type Actor%20Object%20Reference))
  (|CallParentFunction OtherActor) ; This node is disabled and will not be called.\nDrag off pins to build functionality.
)

(event EventTick
  (params (DeltaSeconds :type Float%20%28single-precision%29))
  (|CallParentFunction DeltaSeconds)
  (if (Variables|Default|GetusingPost)
    _))

(event Input|ActionEvents|InputActionSwitchPost
  (params (Key :type Key%20Structure))
  (:Pressed
    (if (not (Variables|Default|GetplayerOne?))
      (if (Variables|Default|GetusingPost)
        (Variables|Default|SetusingPost false)
        (Utilities|IsValid (Variables|Default|GetcurrentPost)
          (:Is%20Valid
            (Variables|/Game/Blueprints/Main_Character_OR_SpaceShip/Player/BP_Post_Test.BP_Post_Test_C|SetisTaken (Variables|Default|GetcurrentPost) false)
            (Variables|/Game/Blueprints/Main_Character_OR_SpaceShip/Player/BP_Post_Test.BP_Post_Test_C|SetplayerOne? (Variables|Default|GetcurrentPost) false)
            (Variables|/Game/Blueprints/Main_Character_OR_SpaceShip/Player/BP_Post_Test.BP_Post_Test_C|SetplayerTwo? (Variables|Default|GetcurrentPost) false)))
        (else
          (for _array_element (Variables|/Game/Blueprints/Main_Character_OR_SpaceShip/Player/BP_Player.BP_Player_C|GetPostList (Variables|Default|GetShip))
            (if (and (not (Variables|/Game/Blueprints/Main_Character_OR_SpaceShip/Player/BP_Post_Test.BP_Post_Test_C|GetisTaken _array_element)) (< (Math|Vector|VectorLength (- (Transformation|GetActorLocation _array_element) (Transformation|GetActorLocation self))) (Variables|Default|GetpostActivationDistance)))
              (bind _output_get (Variables|Default|SetcurrentPost _array_element))
              (Variables|/Game/Blueprints/Main_Character_OR_SpaceShip/Player/BP_Post_Test.BP_Post_Test_C|SetisTaken _output_get true)
              (CallFunction|MovetoPost)
              (Variables|Default|SetusingPost true)
              (if (Variables|Default|GetplayerOne?)
                (Variables|/Game/Blueprints/Main_Character_OR_SpaceShip/Player/BP_Post_Test.BP_Post_Test_C|SetplayerOne? _output_get true)
                (else
                  (Variables|/Game/Blueprints/Main_Character_OR_SpaceShip/Player/BP_Post_Test.BP_Post_Test_C|SetplayerTwo? _output_get true))))))))))

(event Input|ActionEvents|InputActionSwitchPostP2
  (params (Key :type Key%20Structure)))

(event Input|KeyboardEvents|Z
  (params (Key :type Key%20Structure))
  (:Pressed
    (if (not (Variables|Default|GetplayerOne?))
      (if (Variables|Default|GetusingPost)
        (Variables|Default|SetusingPost false)
        (Utilities|IsValid (Variables|Default|GetcurrentPost)
          (:Is%20Valid
            (Variables|/Game/Blueprints/Main_Character_OR_SpaceShip/Player/BP_Post_Test.BP_Post_Test_C|SetisTaken (Variables|Default|GetcurrentPost) false)
            (Variables|/Game/Blueprints/Main_Character_OR_SpaceShip/Player/BP_Post_Test.BP_Post_Test_C|SetplayerOne? (Variables|Default|GetcurrentPost) false)
            (Variables|/Game/Blueprints/Main_Character_OR_SpaceShip/Player/BP_Post_Test.BP_Post_Test_C|SetplayerTwo? (Variables|Default|GetcurrentPost) false)))
        (else
          (for _array_element (Variables|/Game/Blueprints/Main_Character_OR_SpaceShip/Player/BP_Player.BP_Player_C|GetPostList (Variables|Default|GetShip))
            (if (and (not (Variables|/Game/Blueprints/Main_Character_OR_SpaceShip/Player/BP_Post_Test.BP_Post_Test_C|GetisTaken _array_element)) (< (Math|Vector|VectorLength (- (Transformation|GetActorLocation _array_element) (Transformation|GetActorLocation self))) (Variables|Default|GetpostActivationDistance)))
              (bind _output_get (Variables|Default|SetcurrentPost _array_element))
              (Variables|/Game/Blueprints/Main_Character_OR_SpaceShip/Player/BP_Post_Test.BP_Post_Test_C|SetisTaken _output_get true)
              (CallFunction|MovetoPost)
              (Variables|Default|SetusingPost true)
              (if (Variables|Default|GetplayerOne?)
                (Variables|/Game/Blueprints/Main_Character_OR_SpaceShip/Player/BP_Post_Test.BP_Post_Test_C|SetplayerOne? _output_get true)
                (else
                  (Variables|/Game/Blueprints/Main_Character_OR_SpaceShip/Player/BP_Post_Test.BP_Post_Test_C|SetplayerTwo? _output_get true))))))))))

(fn ConstructionScript
  (|CallParentFunction))