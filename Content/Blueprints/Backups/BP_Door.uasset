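; BP_Door is a door actor that opens by destroying itself once enough connections are registered.
; Each Connection? event increments a counter, and reaching the maximum plays a door sound before the actor is removed.
; It also carries apparent enemy leftovers: a game mode reference cached on BeginPlay, an EnemyKilled function for score and explosion effects, and an unused projectile-firing FireNode.
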(event EventBeginPlay
  ;[1 1 1] A supprimer ?
  (bind _asbp_game_mode (Utilities|Casting|CastToBP_GameMode (Game|GetGameMode)))
  (Variables|Default|SetBP_GameMode _asbp_game_mode))

(event EventConnection?
  (Variables|Default|SetNbre (+ (Variables|Default|GetNbre) 1))
  (if (>= (Variables|Default|GetNbre) (Variables|Default|GetNbre_Max))
    (Audio|PlaySound2D "/Game/Assets/Audio/futuristic-door-2.futuristic-door-2" 1.0 1.0 0.0 0 0)
    (Actor|DestroyActor)))

(event EventTick
  (params (DeltaSeconds :type Float%20%28single-precision%29))
  ;[1 1 1] A supprimer ?
)

(fn ConstructionScript)

(fn EnemyKilled
  (bind _returnvalue (Transformation|GetActorLocation))
  (bind _bp_gamemode (Variables|Default|GetBP_GameMode))
  (Effects|SpawnEmitteratLocation "/Game/Assets/Particles/P_Pixel_Explosion_Player.P_Pixel_Explosion_Player" (Transformation|GetActorLocation))
  (Default|EnemyKilled _bp_gamemode)
  (Default|SetScore _bp_gamemode (Variables|Default|GetEnemyScoreValue))
  (Default|PlayCamShake _bp_gamemode "/Game/Blueprints/BP_CamShake.BP_CamShake_C" _returnvalue)
  (Audio|PlaySoundatLocation "/Game/Assets/Audio/Explosion.Explosion" _returnvalue "0, 0, 0" 1.0 1.0 0.0 0 0 0)
  (Actor|DestroyActor))