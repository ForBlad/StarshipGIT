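; BP_Mine is a one-shot proximity mine triggered by the player overlapping its Box component.
; It plays an alert sound, waits briefly, then spawns a BP_Damage_Zone and a large pixel explosion at its location before destroying itself.
; The DoOnce gate precedes the BP_Player cast, so a first overlap by any other actor consumes the trigger without detonating.
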(event OnComponentBeginOverlap(Box)
  (params (OverlappedComponent :type Primitive%20Component%20Object%20Reference) (OtherActor :type Actor%20Object%20Reference) (OtherComp :type Primitive%20Component%20Object%20Reference) (OtherBodyIndex :type Integer) (bFromSweep :type Boolean) (SweepResult :type Hit%20Result%20Structure%20%28by%20ref%29))
  (Utilities|FlowControl|DoOnce false
    (:Completed
      (Utilities|Casting|CastToBP_Player OtherActor)
      (Audio|PlaySoundatLocation "/Game/Assets/Audio/metal-gear-solid-alert.metal-gear-solid-alert" (Transformation|GetActorLocation) "0, 0, 0" 1.0 1.0 0.0 0 0 0)
      (Utilities|FlowControl|Delay 2.0)
      (Game|SpawnActorfromClass "/Game/Blueprints/Backups/BP_Damage_Zone.BP_Damage_Zone_C" (Math|Conversions|ToTransform(Vector) (Transformation|GetActorLocation)) "Undefined" 0 0)
      (Effects|SpawnEmitteratLocation "/Game/Assets/Particles/P_Pixel_Explosion.P_Pixel_Explosion" (Transformation|GetActorLocation) "0, 0, 0" "100.000000,100.000000,100.000000")
      (Actor|DestroyActor))))

(event EventBeginPlay)

(event Collision|EventActorBeginOverlap
  (params (OtherActor :type Actor%20Object%20Reference)))

(event EventTick
  (params (DeltaSeconds :type Float%20%28single-precision%29)))

(fn ConstructionScript)