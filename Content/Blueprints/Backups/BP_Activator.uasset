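; BP_Activator is an enemy actor, stored under Backups, whose setup, movement and firing are disconnected from the empty BeginPlay and Tick events.
; EnemyKilled plays explosion effects, reports kill, score and camera shake to BPGameMode, then destroys the actor, though only unreached setup assigns that reference.
; The FireNode macro spawns a colored projectile after a delay, with player-proximity and trace checks unwired; its only call sits in the dead movement chain.
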(event EventBeginPlay
  ;[1 1 1] Setup References and Variables
)

(event EventTick
  (params (DeltaSeconds :type Float%20%28single-precision%29))
  ;[1 1 1] Movement
)

(fn ConstructionScript)

(fn EnemyKilled
  (bind _returnvalue (Transformation|GetActorLocation))
  (bind _bp_gamemode (Variables|Default|GetBP_GameMode))
  (Effects|SpawnEmitteratLocation "/Game/Assets/Particles/P_Pixel_Explosion_Player.P_Pixel_Explosion_Player" (Transformation|GetActorLocation))
  (Default|EnemyKilled _bp_gamemode)
  (Default|SetScore _bp_gamemode (Variables|Default|GetEnemyScoreValue))
  (Default|PlayCamShake _bp_gamemode "/Game/Blueprints/BP_CamShake.BP_CamShake_C" _returnvalue)
  (Audio|PlaySoundatLocation "/Game/Assets/Audio/Explosion.Explosion" _returnvalue "0, 0, 0" 1.0 1.0 0.0 0 0 0)
  (Actor|DestroyActor))