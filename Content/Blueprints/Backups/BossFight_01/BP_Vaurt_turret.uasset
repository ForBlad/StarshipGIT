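; Boss-fight enemy turret that fires projectiles while the player is inside its detector and registers with the game mode's enemy count.
; Tick drives delayed shots that build Overheat, with a delayed reset and Aiming visibility toggling.
; On death it increments the game instance's destroyed-turret count, calls the boss's shield deactivation, awards score and explodes with camera shake.
; Spawn animation, random movement, rotation and contact damage logic are disconnected.
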(event OnComponentBeginOverlap(player_detector)
  (params (OverlappedComponent :type Primitive%20Component%20Object%20Reference) (OtherActor :type Actor%20Object%20Reference) (OtherComp :type Primitive%20Component%20Object%20Reference) (OtherBodyIndex :type Integer) (bFromSweep :type Boolean) (SweepResult :type Hit%20Result%20Structure%20%28by%20ref%29))
  (Utilities|Casting|CastToBP_Player OtherActor)
  (Variables|Default|Setplayer_in_range true))

(event OnComponentEndOverlap(player_detector)
  (params (OverlappedComponent :type Primitive%20Component%20Object%20Reference) (OtherActor :type Actor%20Object%20Reference) (OtherComp :type Primitive%20Component%20Object%20Reference) (OtherBodyIndex :type Integer))
  (Utilities|Casting|CastToBP_Player OtherActor)
  (Variables|Default|Setplayer_in_range false))

(event EventBeginPlay
  ;[1 1 1] Setup References and Variables
  (bind _asbp_game_mode (Utilities|Casting|CastToBP_GameMode (Game|GetGameMode)))
  (bind _output_get (Variables|Default|SetBP_GameMode _asbp_game_mode))
  (Default|UpdateEnemyCount _output_get 1)
  (bind _asbpi_starship (Utilities|Casting|CastToBPI_Starship (Game|GetGameInstance)))
  (Variables|Default|SetGI_Starship _asbpi_starship))

(event EventTick
  (params (DeltaSeconds :type Float%20%28single-precision%29))
  (Utilities|FlowControl|Sequence
    (:then_0
      (if (> (Variables|Default|Getoverheat) 3.0)
        (Development|SetHiddeninGame (Variables|Default|Getaiming) false true)
        (Utilities|FlowControl|Delay 3.0)
        (Variables|Default|Setoverheat 0.0)))
    (:then_1
      (if (Variables|Default|Getplayer_in_range)
        (if (<= (Variables|Default|Getoverheat) 2e+01)
          (Development|SetHiddeninGame (Variables|Default|Getaiming) true true)
          (|FireNode))))))

(event Game|Damage|EventAnyDamage
  (params (Damage :type Float%20%28single-precision%29) (DamageType :type Damage%20Type%20Object%20Reference) (InstigatedBy :type Controller%20Object%20Reference) (DamageCauser :type Actor%20Object%20Reference))
  (bind _gi_starship (Variables|Default|GetGI_Starship))
  (Variables|Default|SetHealth (Math|Float|Clamp(Float) (- (Variables|Default|GetHealth) Damage) 0.0 (Variables|Default|GetMaxHealth)))
  (if (<= (Variables|Default|GetHealth) 0.0)
    (Variables|/Game/Thibaud/Blueprints/BP_Diverses/BPI_Starship.BPI_Starship_C|SetDestroyed_Turrets _gi_starship (+ (Variables|/Game/Thibaud/Blueprints/BP_Diverses/BPI_Starship.BPI_Starship_C|GetDestroyed_Turrets _gi_starship) 1))
    (bind _returnvalue (Actor|GetActorOfClass "/Game/Thibaud/Blueprints/GPE/BPA_Boss.BPA_Boss_C"))
    (Default|DesactivateShild _returnvalue)
    (CallFunction|EnemyKilled)))

(event Collision|EventHit
  (params (MyComp :type Primitive%20Component%20Object%20Reference) (Other :type Actor%20Object%20Reference) (OtherComp :type Primitive%20Component%20Object%20Reference) (bSelfMoved :type Boolean) (HitLocation :type Vector :default "0, 0, 0") (HitNormal :type Vector :default "0, 0, 0") (NormalImpulse :type Vector :default "0, 0, 0") (Hit :type Hit%20Result%20Structure%20%28by%20ref%29))
  (Utilities|Casting|CastToBP_ProjectilePlayerBase Other
    (:CastFailed
      (Variables|Default|SetMoveDirection (not (Variables|Default|GetMoveDirection))))))

(fn ConstructionScript)

(fn EnemyKilled
  (bind _returnvalue (Transformation|GetActorLocation))
  (bind _bp_gamemode (Variables|Default|GetBP_GameMode))
  (Effects|SpawnEmitteratLocation "/Game/Assets/Particles/Lea_particles/GIGA_EXPLOSION/P_Explosion_3D.P_Explosion_3D" (Transformation|GetActorLocation) "0, 0, 0" "2.000000,2.000000,2.000000")
  (Default|EnemyKilled _bp_gamemode)
  (Default|SetScore _bp_gamemode (Variables|Default|GetEnemyScoreValue))
  (Default|PlayCamShake _bp_gamemode "/Game/Blueprints/BP_CamShake.BP_CamShake_C" _returnvalue)
  (Audio|PlaySoundatLocation "/Game/Assets/Audio/Explosion.Explosion" _returnvalue "0, 0, 0" 1.0 1.0 0.0 0 0 0)
  (Actor|DestroyActor))