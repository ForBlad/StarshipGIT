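; Test turret enemy for the Vaurt boss fight that tracks the player and fires laser projectiles.
; Each Tick re-arms a looping timer and calls Turret directly, snapping rotation toward the player.
; A DoOnce reset after a delay throttles laser spawns from the Scene component to about one per second.
; EnemyKilled plays explosion effects and camera shake, reports the kill and score to the game mode, then destroys the actor.
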(event Custom|Turret
  (bind _asbp_player (Utilities|Casting|CastToBP_Player (Game|Player|GetPlayerPawn 0)))
  (Transformation|SetActorRotation (Math|Rotator|FindLookatRotation (Transformation|GetActorLocation) (Transformation|GetActorLocation _asbp_player)))
  (Utilities|FlowControl|DoOnce false :!label _label
    (:Completed
      (Game|SpawnActorfromClass "/Game/Blueprints/Projectiles/BP_ProjectileEnemyBase_Laser.BP_ProjectileEnemyBase_Laser_C" (Transformation|GetWorldTransform (Variables|Default|GetScene)) "Undefined" 0 "(R=0.820000,G=0.332825,B=0.349142,A=0.000000)" 0)
      (Utilities|FlowControl|Delay 1.0)
      (goto _label Reset))))

(event EventTick
  (params (DeltaSeconds :type Float%20%28single-precision%29))
  (Utilities|Time|SetTimerbyEvent (delegate Custom|Turret) 1.0 true)
  (CallFunction|Turret))

(fn ConstructionScript)

(fn EnemyKilled
  (bind _returnvalue (Transformation|GetActorLocation))
  (bind _bp_gamemode (Variables|Default|GetBP_GameMode))
  (Effects|SpawnEmitteratLocation "/Game/Assets/Particles/Lea_particles/GIGA_EXPLOSION/P_Explosion_3D.P_Explosion_3D" (Transformation|GetActorLocation) "0, 0, 0" "2.000000,2.000000,2.000000")
  (Default|EnemyKilled _bp_gamemode)
  (Default|SetScore _bp_gamemode (Variables|Default|GetEnemyScoreValue))
  (Default|PlayCamShake _bp_gamemode "/Game/Blueprints/BP_CamShake.BP_CamShake_C" _returnvalue)
  (Audio|PlaySoundatLocation "/Game/Assets/Audio/Explosion.Explosion" _returnvalue "0, 0, 0" 1.0 1.0 0.0 0 0 0)
  (Actor|DestroyActor))