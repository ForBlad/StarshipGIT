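; BP_Post_Test_radar is a ship post that switches repair on for whichever of two players occupies it, despite the radar in its name.
; Each Tick it polls IsTaken and uses PlayerOne to set either RepairActive or RepairActiveP2 on the Ship.
; When the post is free it clears both flags every frame.
; BeginPlay, overlap and construction add no logic of their own.
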(event EventBeginPlay
  (|CallParentFunction) ; This node is disabled and will not be called.\nDrag off pins to build functionality.
)

(event Collision|EventActorBeginOverlap
  (params (OtherActor :type Actor%20Object%20Reference))
  (|CallParentFunction OtherActor) ; This node is disabled and will not be called.\nDrag off pins to build functionality.
)

(event EventTick
  (params (DeltaSeconds :type Float%20%28single-precision%29))
  (bind _ship (Variables|Default|GetShip))
  (|CallParentFunction DeltaSeconds)
  (if (Variables|Default|GetisTaken)
    (if (Variables|Default|GetplayerOne?)
      (Variables|/Game/Blueprints/BP_Player.BP_Player_C|SetRepairActive _ship true)
      (else
        (Variables|/Game/Blueprints/BP_Player.BP_Player_C|SetRepairActive_P2 _ship true)))
    (else
      (Variables|/Game/Blueprints/BP_Player.BP_Player_C|SetRepairActive _ship false)
      (Variables|/Game/Blueprints/BP_Player.BP_Player_C|SetRepairActive_P2 _ship false))))

(fn ConstructionScript
  (|CallParentFunction))