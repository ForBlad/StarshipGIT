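; Asteroid enemy that spawns with a random speed and shape and awards score when killed.
; BeginPlay caches BP_GameMode, sets projectile movement initial and max speed to one random value, and randomizes mesh scale independently per axis.
; The construction script applies the stored Scale to the mesh.
; EnemyKilled sends its score value to the game mode, triggers camera shake and sound at its location, then destroys the actor.
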(event EventBeginPlay
  (bind _projectilemovement_0 (Variables|Default|GetProjectileMovement_0))
  (bind _minscale (Variables|Default|GetMinScale))
  (bind _maxscale (Variables|Default|GetMaxScale))
  (bind _returnvalue (Math|Random|RandomFloatinRange _minscale _maxscale))
  (bind _asbp_game_mode (Utilities|Casting|CastToBP_GameMode (Game|GetGameMode)))
  (Variables|Default|SetBP_GameMode _asbp_game_mode)
  (bind _output_get (Variables|Default|SetMoveSpeed (Math|Random|RandomFloatinRange (Variables|Default|GetMinSpeed) (Variables|Default|GetMaxSpeed))))
  (bind _output_get_2 (Variables|/Script/Engine.ProjectileMovementComponent|SetMaxSpeed _projectilemovement_0 _output_get))
  (Variables|/Script/Engine.ProjectileMovementComponent|SetInitialSpeed _projectilemovement_0 _output_get_2)
  (bind _output_get_3 (Variables|Default|SetScale (Math|Vector|MakeVector _returnvalue _returnvalue _returnvalue)))
  (Transformation|SetWorldScale3D (Variables|Default|GetStaticMesh) _output_get_3))

(event Collision|EventActorBeginOverlap
  (params (OtherActor :type Actor%20Object%20Reference)))

(event EventEnemyKilled
  (bind _returnvalue (Transformation|GetActorLocation))
  (bind _bp_gamemode (Variables|Default|GetBP_GameMode))
  (Default|SetScore _bp_gamemode (Variables|Default|GetEnemyScoreValue))
  (Default|PlayCamShake _bp_gamemode 0 _returnvalue)
  (Audio|PlaySoundatLocation 0 _returnvalue "0, 0, 0" 1.0 1.0 0.0 0 0 0)
  (Actor|DestroyActor))

(fn ConstructionScript
  (|CallParentFunction)
  (Transformation|SetWorldScale3D (Variables|Default|GetStaticMesh) (Variables|Default|GetScale)))