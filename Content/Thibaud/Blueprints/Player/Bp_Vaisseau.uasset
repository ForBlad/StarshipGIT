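; Player starship pawn with thrust, yaw steering, two gatling turrets, a rotating laser cannon and a rotatable shield.
; Gatlings turn within yaw limits and spawn projectiles on looping timers; the laser has a three-second cooldown, with CanFire acting as an inverted busy flag.
; A post counter in the game instance (NbreCheckPost) drives timeline camera moves as weapons are taken or released, with separate framing for boss fights.
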(event Custom|Acceleration/Decceleration
  (params (AxisValue :type Float%20%28single-precision%29))
  ;[1 1 1] Movement Physic
  (Pawn|Input|AddMovementInput (Transformation|GetActorRightVector) AxisValue true))

(event Custom|BackWard%20Trust
  (params (Axis%20Value :type Float%20%28single-precision%29))
  ;[1 1 1] Movement Physic
  (Pawn|Input|AddMovementInput (Transformation|GetActorRightVector) Axis%20Value true))

(event Custom|FirecycleRight
  ;[1 1 1] Controle Gatline Droite
  (Game|SpawnActorfromClass "/Game/Thibaud/Blueprints/Player/Balles/Balles.Balles_C" (Transformation|GetWorldTransform (Variables|Default|GetArrow1)) "Undefined" 0 0))

(event Custom|Fire%20Gatling%20Left
  ;[1 1 1] Controle Gatline Gauche
  (Utilities|Time|SetTimerbyEvent (delegate Custom|Firecycle) 0.1 true))

(event Custom|Firecycle
  ;[1 1 1] Controle Gatline Gauche
  (Game|SpawnActorfromClass "/Game/Thibaud/Blueprints/Player/Balles/Balles.Balles_C" (Transformation|GetWorldTransform (Variables|Default|GetArrow)) "Undefined" 0 0))

(event Custom|TurnLeft
  (params (AxisValue :type Float%20%28single-precision%29))
  ;[1 1 1] Ship Rotation
  (if (== AxisValue -1.0)
    (Transformation|AddActorLocalRotation "0,1.000000,0.000000" false false)
    (else
      (Utilities|Time|ClearTimerbyFunctionName 0 "ShipRollLeft")
      (if (== AxisValue 1.0)
        (Transformation|AddActorLocalRotation "0,-1.000000, 0" false false)))))

(event Custom|TurnShield
  (params (AxisValue :type Float%20%28single-precision%29))
  ;[1 1 1] Control Shield
  (if (== AxisValue -1.0)
    (Transformation|AddLocalRotation (Variables|Default|GetBouclier) "0,-1.000000, 0" false false)
    (elif (== AxisValue 1.0)
      (Transformation|AddLocalRotation (Variables|Default|GetBouclier) "0,1.000000, 0" false false))))

(event Custom|TurnRightRotation_GatlineRight
  (params (AxisValue :type Float%20%28single-precision%29))
  (bind _sm_spaceship_09_2_sm_machingun_l (Variables|Default|GetSM_Spaceship_09_2_SM_MachinGun_L))
  (bind _returnvalue (Transformation|GetWorldRotation _sm_spaceship_09_2_sm_machingun_l))
  (bind _yaw (Math|Rotator|BreakRotator _returnvalue))
  ;[1 1 1] Controle Gatline Droite
  (if (== AxisValue -1.0)
    (if (>= _yaw 5.0)
      (Transformation|AddLocalRotation (Variables|Default|GetSM_Spaceship_09_2_SM_MachinGun_L) "0,-1.000000, 0" false false))
    (elif (== AxisValue 1.0)
      (if (<= _yaw 175.0)
        (Transformation|AddLocalRotation (Variables|Default|GetSM_Spaceship_09_2_SM_MachinGun_L) "0,1.000000, 0" false false)))))

(event Custom|LaserTurn
  ;[1 1 1] Turn Big Canon
  (if (not (Variables|Default|GetCanFire?))
    (Game|SpawnActorfromClass "/Game/Thibaud/Blueprints/Player/Balles/Balles_Laser.Balles_Laser_C" (Transformation|GetWorldTransform (Variables|Default|GetArrow2)) "Undefined" 0 0)
    (Variables|Default|SetCanFire? true)
    (Utilities|FlowControl|Delay 3.0)
    (Variables|Default|SetCanFire? false)))

(event Custom|TurnLaser
  (params (AxisValue :type Float%20%28single-precision%29))
  ;[1 1 1] Turn Big Canon
  (if (== AxisValue 1.0)
    (Transformation|AddLocalRotation (Variables|Default|GetSM_Spaceship_09_2_SM_Lazer_BackPIVOTFIX) "0,-1.000000, 0" false false)
    (elif (== AxisValue -1.0)
      (Transformation|AddLocalRotation (Variables|Default|GetSM_Spaceship_09_2_SM_Lazer_BackPIVOTFIX) "0,1.000000, 0" false false))))

(event Custom|TurnLeftRotation_GatlineLeft
  (params (AxisValue :type Float%20%28single-precision%29))
  (bind _sm_spaceship_09_2_sm_machingun_r (Variables|Default|GetSM_Spaceship_09_2_SM_MachinGun_R))
  (bind _returnvalue (Transformation|GetWorldRotation _sm_spaceship_09_2_sm_machingun_r))
  (bind _yaw (Math|Rotator|BreakRotator _returnvalue))
  ;[1 1 1] Controle Gatline Gauche
  (if (== AxisValue -1.0)
    (if (>= _yaw -2e+01)
      (Transformation|AddLocalRotation (Variables|Default|GetSM_Spaceship_09_2_SM_MachinGun_R) "0,-1.000000, 0" false false))
    (elif (== AxisValue 1.0)
      (if (<= _yaw 128.0)
        (Transformation|AddLocalRotation (Variables|Default|GetSM_Spaceship_09_2_SM_MachinGun_R) "0,1.000000, 0" false false)))))

(event Custom|Fire%20Gatling%20Right
  ;[1 1 1] Controle Gatline Droite
  (Utilities|Time|SetTimerbyEvent (delegate Custom|FirecycleRight) 0.1 true))

(event EventBeginPlay
  (bind _asbpi_starship (Utilities|Casting|CastToBPI_Starship (Game|GetGameInstance)))
  (Variables|Default|SetGMI_Starship _asbpi_starship)
  (CallFunction|StartCamera)
  (Game|Player|SetViewTargetwithBlend (Game|GetPlayerController 0) self 0.0 "VTBlend_Linear" 0.0 true))

(event Custom|Modification_Camera_No_Have_Weapon
  (bind _gmi_starship (Variables|Default|GetGMI_Starship))
  (bind _gmi_starship_2 (Variables|Default|GetGMI_Starship))
  (Development|PrintString "Quand le joueur est sur un vaisseau")
  (if (Variables|Default|GetBoss_Camera)
    (Variables|/Game/Thibaud/Blueprints/BP_Diverses/BPI_Starship.BPI_Starship_C|SetNbre_CheckPost _gmi_starship_2 (- (Variables|/Game/Thibaud/Blueprints/BP_Diverses/BPI_Starship.BPI_Starship_C|GetNbre_CheckPost _gmi_starship_2) 1))
    (if (not (>= (Variables|/Game/Thibaud/Blueprints/BP_Diverses/BPI_Starship.BPI_Starship_C|GetNbre_CheckPost (Variables|Default|GetGMI_Starship)) 1))
      (CallFunction|CameraSetupBossNoWeapon))
    (else
      (Variables|/Game/Thibaud/Blueprints/BP_Diverses/BPI_Starship.BPI_Starship_C|SetNbre_CheckPost _gmi_starship (- (Variables|/Game/Thibaud/Blueprints/BP_Diverses/BPI_Starship.BPI_Starship_C|GetNbre_CheckPost _gmi_starship) 1))
      (if (not (>= (Variables|/Game/Thibaud/Blueprints/BP_Diverses/BPI_Starship.BPI_Starship_C|GetNbre_CheckPost (Variables|Default|GetGMI_Starship)) 1))
        (if (not (Variables|Default|GetBoss_Camera))
          (bind _newtrack_0 (Timeline|Zoom/Dezoom Reverse)
            (:Update
              (Transformation|SetRelativeLocation (Variables|Default|GetCamera) _newtrack_0 false false))))))))

(event Custom|Modification_Camera_Have_Weapon
  (bind _gmi_starship (Variables|Default|GetGMI_Starship))
  (bind _gmi_starship_2 (Variables|Default|GetGMI_Starship))
  (if (Variables|Default|GetBoss_Camera)
    (Variables|/Game/Thibaud/Blueprints/BP_Diverses/BPI_Starship.BPI_Starship_C|SetNbre_CheckPost _gmi_starship (+ (Variables|/Game/Thibaud/Blueprints/BP_Diverses/BPI_Starship.BPI_Starship_C|GetNbre_CheckPost _gmi_starship) 1))
    (if (== (Variables|/Game/Thibaud/Blueprints/BP_Diverses/BPI_Starship.BPI_Starship_C|GetNbre_CheckPost (Variables|Default|GetGMI_Starship)) 1)
      (CallFunction|CameraSetupBoss))
    (else
      (Variables|/Game/Thibaud/Blueprints/BP_Diverses/BPI_Starship.BPI_Starship_C|SetNbre_CheckPost _gmi_starship_2 (+ (Variables|/Game/Thibaud/Blueprints/BP_Diverses/BPI_Starship.BPI_Starship_C|GetNbre_CheckPost _gmi_starship_2) 1))
      (Development|PrintString "Quand le joueur est sur un vaisseau")
      (if (not (Variables|Default|GetBoss_Camera))
        (bind _newtrack_0 (Timeline|Zoom/Dezoom Play)
          (:Update
            (Transformation|SetRelativeLocation (Variables|Default|GetCamera) _newtrack_0 false false)))))))

(event Custom|Start_Camera
  (bind _newtrack_0 (Timeline|Zoom/Dezoom Reverse)
    (:Update
      (Transformation|SetRelativeLocation (Variables|Default|GetCamera) _newtrack_0 false false))))

(event Custom|Camera%20Setup%20Boss
  (if (Variables|Default|GetSetup%20Camera%20Start)
    (bind _newtrack_0 (Timeline|Timeline_3 PlayFromStart)
      (:Update
        (Transformation|SetRelativeLocation (Variables|Default|GetCamera) _newtrack_0 false false)))
    (else
      (Variables|Default|SetSetup%20Camera%20Start true)
      (bind _newtrack_0_2 (Timeline|Timeline_1 Play)
        (:Update
          (Transformation|SetRelativeLocation (Variables|Default|GetCamera) _newtrack_0_2 false false))))))

(event Custom|Camera%20Setup%20Boss%20No%20Weapon
  (bind _newtrack_0 (Timeline|Timeline_2 PlayFromStart)
    (:Update
      (Transformation|SetRelativeLocation (Variables|Default|GetCamera) _newtrack_0 false false))))

(fn ConstructionScript)