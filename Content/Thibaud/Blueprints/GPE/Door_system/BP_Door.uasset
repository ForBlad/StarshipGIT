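; BP_Door is a door triggered through its Connection? event, sliding a Cube along a timeline-driven relative location.
; With Timer on, the Delai timeline opens it, waits Timerfloat, then reverses automatically.
; Otherwise, a FlipFlop makes each trigger alternately play or reverse the OuvertureFermeture timeline.
; The Spam flag blocks retriggers mid-cycle, and the construction script applies the Material and animation speed.
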(event Custom|Reverse
  (bind _move (Timeline|Delai Reverse)
    (:Update
      (Variables|Default|SetSpam? true)
      (Transformation|SetRelativeLocation (Variables|Default|GetCube) _move false false))
    (:Finished
      (Utilities|FlowControl|Delay (Variables|Default|GetTimerfloat))
      (Utilities|FlowControl|FlipFlop
        (:A
          (CallFunction|Reverse))
        (:B
          (Variables|Default|SetSpam? false))))))

(event EventConnection?
  (if (Variables|Default|GetTimer?)
    (if (not (Variables|Default|GetSpam?))
      (bind _move (Timeline|Delai PlayFromStart)
        (:Update
          (Variables|Default|SetSpam? true)
          (Transformation|SetRelativeLocation (Variables|Default|GetCube) _move false false))
        (:Finished
          (Utilities|FlowControl|Delay (Variables|Default|GetTimerfloat))
          (Utilities|FlowControl|FlipFlop
            (:A
              (CallFunction|Reverse))
            (:B
              (Variables|Default|SetSpam? false))))))
    (elif (not (Variables|Default|GetSpam?))
      (Utilities|FlowControl|FlipFlop
        (:A
          (bind _move_2 (Timeline|Ouverture/Fermeture Play)
            (:Update
              (Variables|Default|SetSpam? true)
              (Transformation|SetRelativeLocation (Variables|Default|GetCube) _move_2 false false))
            (:Finished
              (Variables|Default|SetSpam? false))))
        (:B
          (Timeline|Ouverture/Fermeture Reverse))))))

(fn ConstructionScript
  (Components|Timeline|SetPlayRate (Variables|Default|GetDelai) (Variables|Default|GetVitesseAnim))
  (Rendering|Material|SetMaterial (Variables|Default|GetCube) 0 (Variables|Default|GetMaterial)))