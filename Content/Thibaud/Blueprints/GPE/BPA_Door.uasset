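; BPA_Door is a door actor that moves its Cube between positions when the Liaison event fires.
; With Timer set, the Delai timeline moves the door, waits Timerfloat seconds, then reverses; a FlipFlop on Finished clears Spam after the return and a second delay.
; Without Timer, a FlipFlop alternates the Normal timeline between forward and reverse on each call.
; A Spam flag blocks retriggering during movement.
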(event Custom|Reverse
  (bind _newtrack_0 (Timeline|Delai Reverse)
    (:Update
      (Variables|Default|SetSpam? true)
      (Transformation|SetRelativeLocation (Variables|Default|GetCube) _newtrack_0 false false))
    (:Finished
      (Utilities|FlowControl|Delay (Variables|Default|GetTimerfloat))
      (Utilities|FlowControl|FlipFlop
        (:A
          (CallFunction|Reverse))
        (:B
          (Variables|Default|SetSpam? false))))))

(event EventLiaison
  (if (Variables|Default|GetTimer?)
    (if (not (Variables|Default|GetSpam?))
      (bind _newtrack_0 (Timeline|Delai PlayFromStart)
        (:Update
          (Variables|Default|SetSpam? true)
          (Transformation|SetRelativeLocation (Variables|Default|GetCube) _newtrack_0 false false))
        (:Finished
          (Utilities|FlowControl|Delay (Variables|Default|GetTimerfloat))
          (Utilities|FlowControl|FlipFlop
            (:A
              (CallFunction|Reverse))
            (:B
              (Variables|Default|SetSpam? false))))))
    (elif (not (Variables|Default|GetSpam?))
      (Utilities|FlowControl|FlipFlop
        (:A
          (bind _newtrack_0_2 (Timeline|Normal PlayFromStart)
            (:Update
              (Variables|Default|SetSpam? true)
              (Transformation|SetRelativeLocation (Variables|Default|GetCube) _newtrack_0_2 false false))
            (:Finished
              (Variables|Default|SetSpam? false))))
        (:B
          (Timeline|Normal Reverse))))))

(fn ConstructionScript)