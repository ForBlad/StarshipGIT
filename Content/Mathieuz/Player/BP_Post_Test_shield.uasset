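; Test shield post for a player on the ship, which flags the Ship's repair state while the post is taken.
; Each Tick, after the parent's Tick, it sets RepairActive for player one or RepairActiveP2 otherwise.
; When the post is free, it clears both flags and cancels the Ship's left and right shield-rotation timers by function name every frame.
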(event EventTick
  (params (DeltaSeconds :type Float%20%28single-precision%29))
  (bind _ship (Variables|Default|GetShip))
  (|CallParentFunction DeltaSeconds)
  (if (Variables|Default|GetisTaken)
    (if (Variables|Default|GetplayerOne?)
      (Variables|/Game/Mathieuz/Player/BP_Player.BP_Player_C|SetRepairActive _ship true)
      (else
        (Variables|/Game/Mathieuz/Player/BP_Player.BP_Player_C|SetRepairActive_P2 _ship true)))
    (else
      (Variables|/Game/Mathieuz/Player/BP_Player.BP_Player_C|SetRepairActive _ship false)
      (Variables|/Game/Mathieuz/Player/BP_Player.BP_Player_C|SetRepairActive_P2 _ship false)
      (Utilities|Time|ClearTimerbyFunctionName _ship "RoateShieldRight")
      (Utilities|Time|ClearTimerbyFunctionName _ship "RotateShieldLeft"))))

(fn ConstructionScript
  (|CallParentFunction))