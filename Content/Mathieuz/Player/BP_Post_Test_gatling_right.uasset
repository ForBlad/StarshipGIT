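; Test version of a player post for the ship's right gatling, usable by player one or two.
; Every Tick, while taken, it sets the Ship's right-gatling active flag for the occupying player.
; While free, it clears both players' gatling and machinegun flags and cancels the Ship's rotation and fire timers by function name.
; Outside Loadout01, it also resets the right missile-fired value after a short delay.
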(event EventBeginPlay
  (|CallParentFunction) ; This node is disabled and will not be called.\nDrag off pins to build functionality.
)

(event Collision|EventActorBeginOverlap
  (params (OtherActor :type Actor%20Object%20Reference))
  (|CallParentFunction OtherActor) ; This node is disabled and will not be called.\nDrag off pins to build functionality.
)

(event EventTick
  (params (DeltaSeconds :type Float%20%28single-precision%29))
  (bind _ship (Variables|Default|GetShip))
  (|CallParentFunction DeltaSeconds)
  (if (Variables|Default|GetisTaken)
    (if (Variables|Default|GetplayerOne?)
      (Variables|/Game/Mathieuz/Player/BP_Player.BP_Player_C|SetGatlingRightActive _ship true)
      (else
        (Variables|/Game/Mathieuz/Player/BP_Player.BP_Player_C|SetGatlingRightActive_P2 _ship true)))
    (else
      (Variables|/Game/Mathieuz/Player/BP_Player.BP_Player_C|SetGatlingRightActive _ship false)
      (Variables|/Game/Mathieuz/Player/BP_Player.BP_Player_C|SetGatlingRightActive_P2 _ship false)
      (Utilities|Time|ClearTimerbyFunctionName _ship "RotateGun")
      (Utilities|Time|ClearTimerbyFunctionName _ship "RotateRightGatling")
      (Utilities|Time|ClearTimerbyFunctionName _ship "RotateRightGatling2")
      (Utilities|Time|ClearTimerbyFunctionName _ship "SecFire")
      (Variables|/Game/Mathieuz/Player/BP_Player.BP_Player_C|SetMachinegun_Right _ship false)
      (Variables|/Game/Mathieuz/Player/BP_Player.BP_Player_C|SetMachinegun_Right_P2 _ship false)
      (if (not (Variables|/Game/Mathieuz/Player/BP_Player.BP_Player_C|GetLoadout_01 _ship))
        (Utilities|FlowControl|Delay 3.0)
        (Variables|/Game/Mathieuz/Player/BP_Player.BP_Player_C|Setmissile_fired_Right _ship 0.0)))))

(fn ConstructionScript
  (|CallParentFunction))