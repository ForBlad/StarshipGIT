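; A player post for the ship's left gatling gun, switching that weapon on for whichever player occupies it.
; Each Tick runs the parent logic, then uses IsTaken and PlayerOne to set the Ship's player-one or player-two gatling flag.
; While the post is free, it clears both players' gatling and machinegun flags and cancels the Ship's fire and rotation timers by function name.
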(event EventTick
  (params (DeltaSeconds :type Float%20%28single-precision%29))
  (bind _ship (Variables|Default|GetShip))
  (|CallParentFunction DeltaSeconds)
  (if (Variables|Default|GetisTaken)
    (if (Variables|Default|GetplayerOne?)
      (Variables|/Game/Mathieuz/Player/BP_Player.BP_Player_C|SetGatlingLeftActive _ship true)
      (else
        (Variables|/Game/Mathieuz/Player/BP_Player.BP_Player_C|SetGatlingLeftActive_P2 _ship true)))
    (else
      (Variables|/Game/Mathieuz/Player/BP_Player.BP_Player_C|SetGatlingLeftActive _ship false)
      (Variables|/Game/Mathieuz/Player/BP_Player.BP_Player_C|SetGatlingLeftActive_P2 _ship false)
      (Utilities|Time|ClearTimerbyFunctionName _ship "SecFire")
      (Utilities|Time|ClearTimerbyFunctionName _ship "RotateGun")
      (Utilities|Time|ClearTimerbyFunctionName _ship "RotateLeftGatling1")
      (Utilities|Time|ClearTimerbyFunctionName _ship "RotateLeftGatling2")
      (Variables|/Game/Mathieuz/Player/BP_Player.BP_Player_C|SetMachinegun_Left _ship false)
      (Variables|/Game/Mathieuz/Player/BP_Player.BP_Player_C|SetMachinegun_Left_P2 _ship false))))

(fn ConstructionScript
  (|CallParentFunction))