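; BP_EnemySmall1 is a work-in-progress small enemy that moves its static mesh along a spline and halts while the player is in range.
; The Move timeline, scaled by PlayRate, maps its alpha to spline distance and restarts when finished.
; PlayerInRange stops the timeline and starts a fast looping timer, never cleared here, that resumes movement once the flag is false.
; Nothing in this graph sets that flag.
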(event Custom|Replay
  (bind _alpha (Timeline|Move PlayFromStart)
    (:Update
      (if (Variables|Default|Getplayer_in_range)
        (CallFunction|Stop)
        (Utilities|Time|SetTimerbyEvent (delegate Custom|Reprise) 0.01 true)
        (else
          (Transformation|SetWorldLocation (Variables|Default|GetStaticMesh) (Spline|GetLocationatDistanceAlongSpline (Variables|Default|GetSpline) (* _alpha (Spline|GetSplineLength (Variables|Default|GetSpline))) "World") false false))))
    (:Finished
      (CallFunction|Replay))))

(event Custom|Check
  (Components|Timeline|SetPlayRate (Variables|Default|GetMove) (Variables|Default|GetPlay%20Rate))
  (bind _alpha (Timeline|Move Play)
    (:Update
      (if (Variables|Default|Getplayer_in_range)
        (CallFunction|Stop)
        (Utilities|Time|SetTimerbyEvent (delegate Custom|Reprise) 0.01 true)
        (else
          (Transformation|SetWorldLocation (Variables|Default|GetStaticMesh) (Spline|GetLocationatDistanceAlongSpline (Variables|Default|GetSpline) (* _alpha (Spline|GetSplineLength (Variables|Default|GetSpline))) "World") false false))))
    (:Finished
      (CallFunction|Replay))))

(event Custom|Stop
  (bind _alpha (Timeline|Move Stop)
    (:Update
      (if (Variables|Default|Getplayer_in_range)
        (CallFunction|Stop)
        (Utilities|Time|SetTimerbyEvent (delegate Custom|Reprise) 0.01 true)
        (else
          (Transformation|SetWorldLocation (Variables|Default|GetStaticMesh) (Spline|GetLocationatDistanceAlongSpline (Variables|Default|GetSpline) (* _alpha (Spline|GetSplineLength (Variables|Default|GetSpline))) "World") false false))))
    (:Finished
      (CallFunction|Replay))))

(event Custom|Reprise
  (if (not (Variables|Default|Getplayer_in_range))
    (CallFunction|Playing)))

(event Custom|Playing
  (bind _alpha (Timeline|Move Play)
    (:Update
      (if (Variables|Default|Getplayer_in_range)
        (CallFunction|Stop)
        (Utilities|Time|SetTimerbyEvent (delegate Custom|Reprise) 0.01 true)
        (else
          (Transformation|SetWorldLocation (Variables|Default|GetStaticMesh) (Spline|GetLocationatDistanceAlongSpline (Variables|Default|GetSpline) (* _alpha (Spline|GetSplineLength (Variables|Default|GetSpline))) "World") false false))))
    (:Finished
      (CallFunction|Replay))))

(event EventBeginPlay
  (|CallParentFunction)
  (CallFunction|Check))

(event Collision|EventActorBeginOverlap
  (params (OtherActor :type Actor%20Object%20Reference)))

(event EventTick
  (params (DeltaSeconds :type Float%20%28single-precision%29))
  (|CallParentFunction DeltaSeconds) ; This node is disabled and will not be called.\nDrag off pins to build functionality.
)

(fn ConstructionScript
  (|CallParentFunction))