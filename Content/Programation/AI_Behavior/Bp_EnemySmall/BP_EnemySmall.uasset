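; Small enemy AI Blueprint that reacts to the player and has impulse-based roaming logic.
; Each Tick, a sphere trace at the actor looks for BP_Player, then rotates the actor along the player-to-enemy direction and moves its mesh toward an offset hit point.
; Four side collision flags feed Ai_Search, a random MultiGate of impulses and turns, which nothing here calls.
; The spline-patrol timeline, which pauses when PlayerInRange, is disconnected from BeginPlay.
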(event OnComponentBeginOverlap(Front_Collision_0)
  (params (OverlappedComponent :type Primitive%20Component%20Object%20Reference) (OtherActor :type Actor%20Object%20Reference) (OtherComp :type Primitive%20Component%20Object%20Reference) (OtherBodyIndex :type Integer) (bFromSweep :type Boolean) (SweepResult :type Hit%20Result%20Structure%20%28by%20ref%29))
  ;[1 0.0498 0.2504] Collision detection
  (Variables|Default|SetOverlapped%20Front_0 true))

(event OnComponentEndOverlap(Front_Collision_0)
  (params (OverlappedComponent :type Primitive%20Component%20Object%20Reference) (OtherActor :type Actor%20Object%20Reference) (OtherComp :type Primitive%20Component%20Object%20Reference) (OtherBodyIndex :type Integer))
  ;[1 0.0498 0.2504] Collision detection
  (Variables|Default|SetOverlapped%20Front_0 false))

(event OnComponentBeginOverlap(Right_Collision_0)
  (params (OverlappedComponent :type Primitive%20Component%20Object%20Reference) (OtherActor :type Actor%20Object%20Reference) (OtherComp :type Primitive%20Component%20Object%20Reference) (OtherBodyIndex :type Integer) (bFromSweep :type Boolean) (SweepResult :type Hit%20Result%20Structure%20%28by%20ref%29))
  ;[1 0.0498 0.2504] Collision detection
  (Variables|Default|SetOverlapped%20Right_0 true))

(event OnComponentEndOverlap(Right_Collision_0)
  (params (OverlappedComponent :type Primitive%20Component%20Object%20Reference) (OtherActor :type Actor%20Object%20Reference) (OtherComp :type Primitive%20Component%20Object%20Reference) (OtherBodyIndex :type Integer))
  ;[1 0.0498 0.2504] Collision detection
  (Variables|Default|SetOverlapped%20Right_0 false))

(event OnComponentBeginOverlap(Left_Collision_0)
  (params (OverlappedComponent :type Primitive%20Component%20Object%20Reference) (OtherActor :type Actor%20Object%20Reference) (OtherComp :type Primitive%20Component%20Object%20Reference) (OtherBodyIndex :type Integer) (bFromSweep :type Boolean) (SweepResult :type Hit%20Result%20Structure%20%28by%20ref%29))
  ;[1 0.0498 0.2504] Collision detection
  (Variables|Default|SetOverlap%20Left_0 true))

(event OnComponentEndOverlap(Left_Collision_0)
  (params (OverlappedComponent :type Primitive%20Component%20Object%20Reference) (OtherActor :type Actor%20Object%20Reference) (OtherComp :type Primitive%20Component%20Object%20Reference) (OtherBodyIndex :type Integer))
  ;[1 0.0498 0.2504] Collision detection
  (Variables|Default|SetOverlap%20Left_0 false))

(event OnComponentBeginOverlap(Rear_Collision_0)
  (params (OverlappedComponent :type Primitive%20Component%20Object%20Reference) (OtherActor :type Actor%20Object%20Reference) (OtherComp :type Primitive%20Component%20Object%20Reference) (OtherBodyIndex :type Integer) (bFromSweep :type Boolean) (SweepResult :type Hit%20Result%20Structure%20%28by%20ref%29))
  ;[1 0.0498 0.2504] Collision detection
  (Variables|Default|SetOverlap%20Rear_0 true))

(event OnComponentEndOverlap(Rear_Collision_0)
  (params (OverlappedComponent :type Primitive%20Component%20Object%20Reference) (OtherActor :type Actor%20Object%20Reference) (OtherComp :type Primitive%20Component%20Object%20Reference) (OtherBodyIndex :type Integer))
  ;[1 0.0498 0.2504] Collision detection
  (Variables|Default|SetOverlap%20Rear_0 false))

(event Custom|Ai_Search
  ;[1 1 1] AI Roaming
  (Utilities|FlowControl|MultiGate true true 0
    (:Out%200
      (if (Variables|Default|GetOverlapped%20Front_0)
        (CallFunction|Rotate)
        (CallFunction|GoForward)
        (else
          (CallFunction|ConstForwarding)
          (CallFunction|ConstRotation))))
    (:Out%201
      (if (Variables|Default|GetOverlapped%20Right_0)
        (CallFunction|GoRight)
        (else
          (CallFunction|GoLeft))))
    (:Out%202
      (if (Variables|Default|GetOverlap%20Left_0)
        (CallFunction|GoLeft)
        (else
          (CallFunction|GoRight))))
    (:Out%203
      (if (Variables|Default|GetOverlap%20Rear_0)
        (CallFunction|GoRear)))))

(event Custom|Replay
  (bind _alpha (Timeline|Move PlayFromStart)
    (:Update
      (if (Variables|Default|Getplayer_in_range)
        (CallFunction|Stop)
        (Utilities|Time|SetTimerbyEvent (delegate Custom|Reprise) 0.01 true)
        (else
          (Transformation|SetWorldLocation (Variables|Default|GetStaticMesh) (Spline|GetLocationatDistanceAlongSpline (Variables|Default|GetSpline) (* _alpha (Spline|GetSplineLength (Variables|Default|GetSpline))) "World") false false))))
    (:Finished
      (CallFunction|Replay))))

(event Custom|Go%20Right
  (bind _staticmesh (Variables|Default|GetStaticMesh))
  ;[1 1 1] Movements
  (Physics|AddImpulse _staticmesh (* (Math|Vector|GetForwardVector _staticmesh) 3e+01) "None" true))

(event Custom|Go%20Forward
  (bind _staticmesh (Variables|Default|GetStaticMesh))
  ;[1 1 1] Movements
  (Physics|AddImpulse _staticmesh (* (Math|Vector|GetForwardVector _staticmesh) -3e+01) "None" true))

(event Custom|Go%20Rear
  (bind _staticmesh (Variables|Default|GetStaticMesh))
  ;[1 1 1] Movements
  (Physics|AddImpulse _staticmesh (* (Math|Vector|GetForwardVector _staticmesh) -3e+01) "None" true))

(event Custom|Rotate
  (bind _staticmesh (Variables|Default|GetStaticMesh))
  (bind _returnvalue (Transformation|GetWorldRotation _staticmesh))
  ;[1 1 1] Movements
  (Transformation|SetWorldRotation _staticmesh (Math|Rotator|MakeRotator (.roll _returnvalue) (+ (.pitch _returnvalue) 1.8e+02) (.yaw _returnvalue)) false false))

(event Custom|Check
  (Components|Timeline|SetPlayRate (Variables|Default|GetMove) (Variables|Default|GetPlay%20Rate))
  (bind _alpha (Timeline|Move Play)
    (:Update
      (if (Variables|Default|Getplayer_in_range)
        (CallFunction|Stop)
        (Utilities|Time|SetTimerbyEvent (delegate Custom|Reprise) 0.01 true)
        (else
          (Transformation|SetWorldLocation (Variables|Default|GetStaticMesh) (Spline|GetLocationatDistanceAlongSpline (Variables|Default|GetSpline) (* _alpha (Spline|GetSplineLength (Variables|Default|GetSpline))) "World") false false))))
    (:Finished
      (CallFunction|Replay))))

(event Custom|Stop
  (bind _alpha (Timeline|Move Stop)
    (:Update
      (if (Variables|Default|Getplayer_in_range)
        (CallFunction|Stop)
        (Utilities|Time|SetTimerbyEvent (delegate Custom|Reprise) 0.01 true)
        (else
          (Transformation|SetWorldLocation (Variables|Default|GetStaticMesh) (Spline|GetLocationatDistanceAlongSpline (Variables|Default|GetSpline) (* _alpha (Spline|GetSplineLength (Variables|Default|GetSpline))) "World") false false))))
    (:Finished
      (CallFunction|Replay))))

(event Custom|Reprise
  (if (not (Variables|Default|Getplayer_in_range))
    (CallFunction|Playing)))

(event Custom|Playing
  (bind _alpha (Timeline|Move Play)
    (:Update
      (if (Variables|Default|Getplayer_in_range)
        (CallFunction|Stop)
        (Utilities|Time|SetTimerbyEvent (delegate Custom|Reprise) 0.01 true)
        (else
          (Transformation|SetWorldLocation (Variables|Default|GetStaticMesh) (Spline|GetLocationatDistanceAlongSpline (Variables|Default|GetSpline) (* _alpha (Spline|GetSplineLength (Variables|Default|GetSpline))) "World") false false))))
    (:Finished
      (CallFunction|Replay))))

(event Custom|Go%20Left
  (bind _staticmesh (Variables|Default|GetStaticMesh))
  ;[1 1 1] Movements
  (Physics|AddImpulse _staticmesh (* (Math|Vector|GetForwardVector _staticmesh) -3e+01) "None" true))

(event Custom|Const%20Forwarding
  (bind _staticmesh (Variables|Default|GetStaticMesh))
  ;[1 1 1] Constant Movements
  (Physics|AddImpulse _staticmesh (* (Math|Vector|GetForwardVector _staticmesh) (Math|Random|RandomFloatinRange 7e+01 3e+02)) "None" false))

(event Custom|Const%20Rotation
  (bind _staticmesh (Variables|Default|GetStaticMesh))
  (bind _returnvalue (Transformation|GetWorldRotation _staticmesh))
  ;[1 1 1] Constant Movements
  (Transformation|SetWorldRotation _staticmesh (Math|Rotator|MakeRotator (.roll _returnvalue) (.pitch _returnvalue) (+ (.yaw _returnvalue) (Variables|Default|GetConst%20Rotation%20Rate_0))) false false)
  (Utilities|FlowControl|Delay 27.0)
  (Utilities|FlowControl|MultiGate true false -1
    (:Out%200
      (Variables|Default|SetConst%20Rotation%20Rate_0 1.5))
    (:Out%201
      (Variables|Default|SetConst%20Rotation%20Rate_0 -1.5))))

(event EventBeginPlay)

(event Collision|EventActorBeginOverlap
  (params (OtherActor :type Actor%20Object%20Reference)))

(event EventTick
  (params (DeltaSeconds :type Float%20%28single-precision%29))
  (bind _returnvalue (Transformation|GetActorLocation))
  ;[1 1 1] Collision Behavior
  (bind _outactors (Actor|GetAllActorsOfClass "/Script/Engine.StaticMeshActor"))
  (bind _outhit (Collision|SphereTraceByChannel _returnvalue _returnvalue 0.0 "TraceTypeQuery1" false _outactors "None"))
  (if (Utilities|Enum|Equal(Enum) (Utilities|GetDisplayName (.HitActor (Collision|BreakHitResult _outhit))) "BP_Player")
    (bind _asbp_player (Utilities|Casting|CastToBP_Player (.HitActor (Collision|BreakHitResult _outhit))))
    (Transformation|SetActorRotation (Math|Rotator|FindLookatRotation (Transformation|GetActorLocation _asbp_player) (Transformation|GetActorLocation)))
    (Components|MoveComponentTo (Variables|Default|GetStaticMesh) (Math|Vector|MakeVector (.X (Math|Vector|BreakVector (- (.ImpactPoint (Collision|BreakHitResult _outhit)) "150.000000,150.000000, 0"))) (.Y (Math|Vector|BreakVector (- (.ImpactPoint (Collision|BreakHitResult _outhit)) "150.000000,150.000000, 0"))) (.Z (Math|Vector|BreakVector (- (.ImpactPoint (Collision|BreakHitResult _outhit)) "150.000000,150.000000, 0")))) "0, 0, 0" true true 0.2 false)))

(fn ConstructionScript
  (|CallParentFunction))