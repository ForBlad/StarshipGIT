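; VAURTE boss enemy that descends on spawn, then fires missiles while the player is inside its detection volume.
; A Tick-driven Delay re-arms the missile every four seconds; side-to-side movement logic is present but unwired.
; A second trigger adds the fight widget and starts boss music.
; At zero health it chains explosions, reports kill and score to BP_GameMode, destroys itself and creates, without displaying, a victory widget.
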(event OnComponentBeginOverlap(player_detector)
  (params (OverlappedComponent :type Primitive%20Component%20Object%20Reference) (OtherActor :type Actor%20Object%20Reference) (OtherComp :type Primitive%20Component%20Object%20Reference) (OtherBodyIndex :type Integer) (bFromSweep :type Boolean) (SweepResult :type Hit%20Result%20Structure%20%28by%20ref%29))
  (Utilities|Casting|CastToBP_Player OtherActor)
  (Variables|Default|Setplayer_in_range true))

(event OnComponentEndOverlap(player_detector)
  (params (OverlappedComponent :type Primitive%20Component%20Object%20Reference) (OtherActor :type Actor%20Object%20Reference) (OtherComp :type Primitive%20Component%20Object%20Reference) (OtherBodyIndex :type Integer))
  (Utilities|Casting|CastToBP_Player OtherActor)
  (Variables|Default|Setplayer_in_range false))

(event OnComponentBeginOverlap(bossfight_detector)
  (params (OverlappedComponent :type Primitive%20Component%20Object%20Reference) (OtherActor :type Actor%20Object%20Reference) (OtherComp :type Primitive%20Component%20Object%20Reference) (OtherBodyIndex :type Integer) (bFromSweep :type Boolean) (SweepResult :type Hit%20Result%20Structure%20%28by%20ref%29))
  (Utilities|Casting|CastToBP_Player OtherActor)
  (bind _returnvalue (UserInterface|CreateWidget "/Game/Blueprints/Main_Character_OR_SpaceShip/Player/Widgets/BPW_VAURT_fight.BPW_VAURT_fight_C"))
  (UserInterface|Viewport|AddtoViewport _returnvalue 0)
  (Utilities|FlowControl|DoOnce false
    (:Completed
      (Audio|PlaySoundatLocation "/Game/Assets/Audio/dark-souls-iii-soundtrack-ost-vordt-of-the-boreal-valley_1_.dark-souls-iii-soundtrack-ost-vordt-of-the-boreal-valley_1_" "0, 0, 0" "0, 0, 0" 1.0 1.0 0.0 0 0 0))))

(event EventBeginPlay
  ;[1 1 1] Setup References and Variables
  (bind _asbp_game_mode (Utilities|Casting|CastToBP_GameMode (Game|GetGameMode)))
  (bind _output_get (Variables|Default|SetBP_GameMode _asbp_game_mode))
  (Default|UpdateEnemyCount _output_get 1)
  (Variables|Default|SetMoveDirection (Math|Random|RandomBool))
  (Variables|Default|SetMoveSpeed (Math|Random|RandomFloatinRange (Variables|Default|GetMinSpeed) (Variables|Default|GetMaxSpeed)))
  (Variables|Default|SetSpawnLocation (Transformation|GetActorLocation))
  ;[1 1 1] SpawnAnimation
  (bind _entryspeed (Timeline|SpawnAnimation Play)
    (:Update
      (Transformation|SetActorLocation (Math|Vector|Lerp(Vector) (Variables|Default|GetSpawnLocation) (- (Variables|Default|GetSpawnLocation) "0, 0,120.000000") _entryspeed) false false))
    (:Finished
      (Variables|Default|SetMoveEnabled true))))

(event EventTick
  (params (DeltaSeconds :type Float%20%28single-precision%29))
  ;[1 1 1] Movement
  (Utilities|FlowControl|Sequence
    (:then_0
      (if (Variables|Default|Getplayer_in_range)
        (if (Variables|Default|GetMissile_Ready)
          (|FireNode))))
    (:then_1
      (Utilities|FlowControl|Delay 4.0)
      (Variables|Default|SetMissile_ready true))))

(event Game|Damage|EventAnyDamage
  (params (Damage :type Float%20%28single-precision%29) (DamageType :type Damage%20Type%20Object%20Reference) (InstigatedBy :type Controller%20Object%20Reference) (DamageCauser :type Actor%20Object%20Reference))
  (Variables|Default|SetHealth (Math|Float|Clamp(Float) (- (Variables|Default|GetHealth) Damage) 0.0 (Variables|Default|GetMaxHealth)))
  (if (<= (Variables|Default|GetHealth) 0.0)
    (Utilities|FlowControl|Delay 0.2)
    (Effects|SpawnEmitteratLocation "/Game/InfinityBladeEffects/Effects/FX_Mobile/combat/P_Impact_Golem_Gib_Fire.P_Impact_Golem_Gib_Fire" (Transformation|GetActorLocation) "0, 0, 0" "10.000000,10.000000,10.000000")
    (Utilities|FlowControl|Delay 0.5)
    (Effects|SpawnEmitteratLocation "/Game/InfinityBladeEffects/Effects/FX_Mobile/combat/P_Impact_Golem_Gib_Fire.P_Impact_Golem_Gib_Fire" (Transformation|GetActorLocation) "0, 0, 0" "10.000000,10.000000,10.000000")
    (Utilities|FlowControl|Delay 0.5)
    (Effects|SpawnEmitteratLocation "/Game/InfinityBladeEffects/Effects/FX_Mobile/combat/P_Impact_Golem_Gib_Fire.P_Impact_Golem_Gib_Fire" (Transformation|GetActorLocation) "0, 0, 0" "10.000000,10.000000,10.000000")
    (Utilities|FlowControl|Delay 0.5)
    (Effects|SpawnEmitteratLocation "/Game/InfinityBladeEffects/Effects/FX_Mobile/combat/P_Impact_Golem_Gib_Fire.P_Impact_Golem_Gib_Fire" (Transformation|GetActorLocation) "0, 0, 0" "10.000000,10.000000,10.000000")
    (Utilities|FlowControl|Delay 0.5)
    (Effects|SpawnEmitteratLocation "/Game/InfinityBladeEffects/Effects/FX_Mobile/combat/P_Impact_Golem_Gib_Fire.P_Impact_Golem_Gib_Fire" (Transformation|GetActorLocation) "0, 0, 0" "10.000000,10.000000,10.000000")
    (Variables|Default|SetVaurte_isDead true)
    (CallFunction|EnemyKilled)))

(event Collision|EventHit
  (params (MyComp :type Primitive%20Component%20Object%20Reference) (Other :type Actor%20Object%20Reference) (OtherComp :type Primitive%20Component%20Object%20Reference) (bSelfMoved :type Boolean) (HitLocation :type Vector :default "0, 0, 0") (HitNormal :type Vector :default "0, 0, 0") (NormalImpulse :type Vector :default "0, 0, 0") (Hit :type Hit%20Result%20Structure%20%28by%20ref%29))
  (Utilities|Casting|CastToBP_ProjectilePlayerBase Other
    (:CastFailed
      (Variables|Default|SetMoveDirection (not (Variables|Default|GetMoveDirection))))))

(fn ConstructionScript)

(fn EnemyKilled
  (bind _returnvalue (Transformation|GetActorLocation))
  (bind _bp_gamemode (Variables|Default|GetBP_GameMode))
  (Effects|SpawnEmitteratLocation "/Game/Assets/Particles/Lea_particles/GIGA_EXPLOSION/P_Explosion_3D.P_Explosion_3D" (Transformation|GetActorLocation) "0, 0, 0" "4.000000,4.000000,4.000000")
  (Default|EnemyKilled _bp_gamemode)
  (Default|SetScore _bp_gamemode (Variables|Default|GetEnemyScoreValue))
  (Default|PlayCamShake _bp_gamemode "/Game/Blueprints/BP_CamShake.BP_CamShake_C" _returnvalue)
  (Audio|PlaySoundatLocation "/Game/Assets/Audio/Explosion.Explosion" _returnvalue "0, 0, 0" 1.0 1.0 0.0 0 0 0)
  (Actor|DestroyActor)
  (UserInterface|CreateWidget "/Game/Blueprints/Main_Character_OR_SpaceShip/Player/Widgets/BPW_bossbeaten.BPW_bossbeaten_C"))