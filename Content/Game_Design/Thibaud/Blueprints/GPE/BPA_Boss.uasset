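; Boss actor whose shields drop once enough of its turrets have been destroyed.
; On BeginPlay it caches the game instance cast to BPI_Starship to read the shared destroyed-turret count.
; Desactivate_Shild checks that count and, once five or more turrets are down, destroys all three shield components.
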(event Custom|Desactivate_Shild
  (if (>= (Variables|/Game/Game_Design/Thibaud/Blueprints/BP_Diverses/BPI_Starship.BPI_Starship_C|GetDestroyed_Turrets (Variables|Default|GetGI_Starship)) 5)
    (Components|DestroyComponent (Variables|Default|GetShield1))))

(event EventBeginPlay
  (bind _asbpi_starship (Utilities|Casting|CastToBPI_Starship (Game|GetGameInstance)))
  (Variables|Default|SetGI_Starship _asbpi_starship))

(fn ConstructionScript)